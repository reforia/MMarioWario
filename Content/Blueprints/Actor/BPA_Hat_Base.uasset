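; Base thrown-hat actor that flies out from the player, hovers, then flies back, reporting possession and jump opportunities.
; Looping timers drive forward flight to a max distance and the homing return, which disables collision.
; A repeating sphere trace fires dispatchers for BPI_Possessable pawns, player contact while hovering, or blocking objects, which end flight early.
; A one-shot timer ends the hover; a dispatcher signals arrival at the player.
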(event Custom|LaunchHat
  (params (Player :type Char%20Player%20Base%20Object%20Reference))
  (bind _output_get (Variables|Default|SetCallerPlayer Player))
  (if (Utilities|IsValid _output_get)
    (Variables|Default|SetInitialLocation (Transformation|GetActorLocation))
    (bind _returnvalue (Utilities|Time|SetTimerbyEvent (delegate Custom|HatFlyingTick) 0.016667 true))
    (Variables|Default|SetFlyingTimerDelegateHandle _returnvalue)
    (bind _returnvalue_2 (Utilities|Time|SetTimerbyEvent (delegate Custom|CheckingStayingOverlap) 0.03 true))
    (Variables|Default|SetHatStayTickTimerDelegateHandle _returnvalue_2)))

(event Custom|CheckingStayingOverlap
  (bind _returnvalue (Transformation|GetActorLocation))
  (bind _outhit (Collision|SphereTraceForObjects _returnvalue _returnvalue 64.0 (Utilities|Array|MakeArray "ObjectTypeQuery1" "ObjectTypeQuery2" "ObjectTypeQuery3" "ObjectTypeQuery4" "ObjectTypeQuery5" "ObjectTypeQuery6") false 0 "ForDuration"))
  (if (.binitialoverlap _outhit)
    (Development|PrintString (Utilities|GetDisplayName (.hitactor _outhit)))
    (if (!= (.hitactor _outhit) (Variables|Default|GetCallerPlayer))
      (if (Utilities|DoesObjectImplementInterface (.hitactor _outhit) "/Game/Blueprints/Controller/BPI_Possessable.BPI_Possessable_C")
        (bind _aspawn (Utilities|Casting|CastToPawn (.hitactor _outhit)))
        (Default|CallOnHatReachedPossessablePawn _aspawn)
        (else
          (Default|CallOnHatBlockedbyWorldObject)
          (Utilities|Time|ClearandInvalidateTimerbyHandle (Variables|Default|GetFlyingTimerDelegateHandle))
          (if (not (Variables|Default|GetIsHatStaying))
            (CallFunction|HatStay))))
      (elif (Variables|Default|GetIsHatStaying)
        (Default|CallOnHatBeingJumpedbyPlayer)))))

(event Custom|HatFlyingTick
  (Transformation|AddActorWorldOffset (* (Transformation|GetActorForwardVector) (Variables|Default|GetHatFlyingSpeed)) true)
  (if (>= (Math|Vector|Distance2D(Vector) (Transformation|GetActorLocation) (Variables|Default|GetInitialLocation)) (Variables|Default|GetMaxFlyingDistance))
    (Utilities|Time|ClearandInvalidateTimerbyHandle (Variables|Default|GetFlyingTimerDelegateHandle))
    (CallFunction|HatStay)))

(event Custom|HatStay
  (Variables|Default|SetIsHatStaying true)
  (bind _returnvalue (Utilities|Time|SetTimerbyEvent (delegate Custom|HatReturn) (Variables|Default|GetHatStayTime)))
  (Variables|Default|SetHatStayTimerDelegateHandle _returnvalue))

(event Custom|HatReturn
  (Utilities|Time|ClearandInvalidateTimerbyHandle (Variables|Default|GetHatStayTickTimerDelegateHandle))
  (Variables|Default|SetIsHatStaying false)
  ;[1 1 1] Ignore Collisions
  (Collision|SetActorEnableCollision false)
  (Variables|Default|GetCallerPlayer
    (:then
      (bind _returnvalue (Utilities|Time|SetTimerbyEvent (delegate Custom|FlyingBackToPlayerTick) 0.016667 true))
      (Variables|Default|SetFlyingBackToPlayerTimerHandle _returnvalue))
    (:else
      (Development|PrintString "Player Not Valid!!! Destroying the hat itself")
      (Actor|DestroyActor))))

(event Custom|FlyingBackToPlayerTick
  (bind _callerplayer (Variables|Default|GetCallerPlayer)
    (:then
      (if (<= (Math|Vector|Distance(Vector) (Transformation|GetActorLocation _callerplayer) (Transformation|GetActorLocation)) 1e+02)
        (Utilities|Time|ClearandInvalidateTimerbyHandle (Variables|Default|GetFlyingBackToPlayerTimerHandle))
        (Default|CallOnHatReturned)
        (else
          (Transformation|AddActorWorldOffset (* (Math|Vector|Normalize (- (Transformation|GetActorLocation (Variables|Default|GetCallerPlayer)) (Transformation|GetActorLocation))) (Variables|Default|GetFlyingBackSpeed)) true))))
    (:else
      (Development|PrintString "Player Not Valid!!! Destroying the hat itself")
      (Actor|DestroyActor))))

(event EventBeginPlay)

(event Collision|EventActorBeginOverlap
  (params (OtherActor :type Actor%20Object%20Reference)))

(event EventTick
  (params (DeltaSeconds :type Float%20%28single-precision%29)))

(fn ConstructionScript)