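; Trigger-response bridge actor that falls down when triggered and returns when reset.
; The ControllerTriggered event waits a configurable delay, then plays the BridgetFallDown timeline; a reset reverses it immediately.
; The timeline's LowerRate track drives a rotator lerp that swings the root's relative rotation from a 90-degree offset to zero.
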(event EventBeginPlay
  (|CallParentFunction) ; This node is disabled and will not be called.\nDrag off pins to build functionality.
)

(event Collision|EventActorBeginOverlap
  (params (OtherActor :type Actor%20Object%20Reference))
  (|CallParentFunction OtherActor) ; This node is disabled and will not be called.\nDrag off pins to build functionality.
)

(event EventTick
  (params (DeltaSeconds :type Float%20%28single-precision%29))
  (|CallParentFunction DeltaSeconds) ; This node is disabled and will not be called.\nDrag off pins to build functionality.
)

(event EventControllerTriggered
  (params (TriggerOrReset :type Boolean))
  (if TriggerOrReset
    (Utilities|FlowControl|Delay (Variables|Default|GetTriggerDelay))
    (bind _lowerrate (Timeline|BridgetFallDown Play)
      (:Update
        (Transformation|SetRelativeRotation (Variables|Default|GetRoot) (Math|Rotator|Lerp(Rotator) "90.000000, 0, 0" "0, 0, 0" _lowerrate) false false)))
    (else
      (Timeline|BridgetFallDown Reverse))))

(fn ConstructionScript
  (|CallParentFunction))