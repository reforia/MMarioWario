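; Base player character for a Mario Odyssey-style platformer, with camera-relative movement, jump, wall jump, ground smash, forward roll and a throwable hat.
; Control scheme changes from PC_PlayerBase drive gravity and reset smash and roll states.
; The spawned hat reports back through delegates for hat jumps and pawn capture, where the hidden character glides to the target, possesses it and destroys itself.
; Tick auto-aligns the spring arm camera using game instance settings.
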(event Custom|OnHatReturned)

(event Custom|PerformHatJump
  (CallFunction|ResetRollForward)
  (Character|LaunchCharacter (* (Math|Vector|Normalize (+ (Transformation|GetActorForwardVector) (Math|Vector|MakeVector 0.0 0.0 (Variables|Hat|GetHatLaunchZ)))) (Variables|Hat|GetHatLaunchForce)) true true)
  (Development|PrintString "Player Hat Jumped"))

(event Custom|ResetSmashControlSchemeListener
  (params (NewControlScheme :type Enum_ControlScheme%20Enum :default "NewEnumerator0"))
  (if (Utilities|Enum|Equal(Enum) NewControlScheme "NewEnumerator0")
    (Variables|Smash|SetInSmash false)
    (EventDispatchers|UnbindEventfromOnControlSchemeChanged (stale EventSmash _controllerref) (delegate Custom|ResetSmashControlSchemeListener))
    (Utilities|FlowControl|Delay (Variables|Smash|GetSmashStunDuration))
    (Input|SetIgnoreMoveInput (stale EventSmash _controllerref) false)))

(event Custom|ControlSchemeChanged
  (params (NewControlScheme :type Enum_ControlScheme%20Enum :default "NewEnumerator0"))
  (bind _charactermovement (Variables|Character|GetCharacterMovement))
  (switch Utilities|FlowControl|Switch|SwitchonEnum_ControlScheme NewControlScheme
    (:NewEnumerator0
      (Variables|/Script/Engine.CharacterMovementComponent|SetGravityScale _charactermovement (Variables|Jump|GetBaseJumpingGravityFactor) :!label _label))
    (:NewEnumerator1
      (goto _label))
    (:NewEnumerator2
      (Components|Movement|StopMovementImmediately _charactermovement)
      (Variables|/Script/Engine.CharacterMovementComponent|SetGravityScale _charactermovement 0.0)
      (Character|StopJumping))))

(event Custom|RollForwardResetStatusListener
  (params (NewControlScheme :type Enum_ControlScheme%20Enum :default "NewEnumerator0"))
  (switch Utilities|FlowControl|Switch|SwitchonEnum_ControlScheme NewControlScheme
    (:NewEnumerator0
      _)
    (:NewEnumerator3
      _)
    (:NewEnumerator2
      _))
  (CallFunction|ResetRollForward)
  (EventDispatchers|UnbindEventfromOnControlSchemeChanged (stale EventRollForward _controllerref) (delegate Custom|RollForwardResetStatusListener)))

(event Custom|TryPossessPawn
  (params (Pawn :type Pawn%20Object%20Reference))
  (bind _controllerref (Variables|Default|GetControllerRef))
  (EventDispatchers|UnbindEventfromOnHatReachedPossessablePawn (Variables|Hat|GetHatRef) (delegate Custom|TryPossessPawn))
  (Variables|/Script/Engine.SpringArmComponent|SetbDoCollisionTest (Variables|Default|GetSpringArm) true)
  (Input|SetIgnoreLookInput _controllerref true)
  (Input|SetIgnoreMoveInput _controllerref true)
  (Variables|/Script/Engine.CharacterMovementComponent|SetGravityScale (Variables|Character|GetCharacterMovement) 0.0)
  (Rendering|SetActorHiddenInGame true)
  (Rendering|SetActorHiddenInGame (Variables|Hat|GetHatRef) true)
  (Collision|SetActorEnableCollision false)
  (Collision|SetActorEnableCollision (Variables|Hat|GetHatRef) false)
  (Components|Movement|StopMovementImmediately (Variables|Character|GetCharacterMovement))
  (bind _returnvalue (Utilities|Time|SetTimerbyEvent (delegate Custom|AccessingPossessableActor) (Utilities|Time|GetWorldDeltaSeconds) true))
  (Variables|Default|SetAccessingPossessableCharacterTimeHandle _returnvalue))

(event Custom|AccessingPossessableActor
  (bind _returnvalue (Transformation|GetActorLocation))
  (if (<= (Math|Vector|Distance(Vector) _returnvalue (Transformation|GetActorLocation (stale Custom|TryPossessPawn Pawn))) 8e+01)
    (Utilities|Time|ClearandInvalidateTimerbyHandle (Variables|Default|GetAccessingPossessableCharacterTimeHandle))
    (CallFunction|TryPossessTarget (stale Custom|TryPossessPawn Pawn))
    (Utilities|FlowControl|Delay 3.0)
    (Actor|DestroyActor)
    (else
      (Transformation|SetActorLocation (Math|Interpolation|VInterpTo _returnvalue (Transformation|GetActorLocation (stale Custom|TryPossessPawn Pawn)) (Utilities|Time|GetWorldDeltaSeconds) 2.0) true false))))

(event EventBeginPlay
  ;[1 1 1] HACK Give player a hat
  (bind _returnvalue (Game|SpawnActorfromClass "/Game/Blueprints/Actor/BPA_Hat_Base.BPA_Hat_Base_C" (Math|Transform|MakeTransform "0, 0, 0" "0, 0, 0" "1.000000,1.000000,1.000000") "AlwaysSpawn" 0 self))
  (Variables|Hat|SetHatRef _returnvalue)
  (CallFunction|InitializeCameraRotation))

(event Collision|EventActorBeginOverlap
  (params (OtherActor :type Actor%20Object%20Reference)))

(event EventRollForward
  (params (rollInputDir :type Vector%202D%20Structure))
  (if (CallFunction|CanRollForward)
    (Variables|RollFoward|SetInRollForward true)
    (Character|LaunchCharacter (* (+ (Transformation|GetActorForwardVector) "0.000000,0,0.600000") (Variables|RollFoward|GetRollForwardForce)) false true)
    (bind _controllerref (Variables|Default|GetControllerRef)
      (:then
        (EventDispatchers|BindEventtoOnControlSchemeChanged _controllerref (delegate Custom|RollForwardResetStatusListener)))
      (:else))))

(event EventLaunchHat
  (bind _charactermovement (Variables|Character|GetCharacterMovement))
  (bind _hatref (Variables|Hat|GetHatRef))
  (if (Variables|/Game/Blueprints/Actor/BPA_Hat_Base.BPA_Hat_Base_C|GetIsHatReady _hatref)
    (if (CallFunction|CanTriggerHat)
      (if (AI|Components|NavMovement|IsMovingonGround (Variables|Character|GetCharacterMovement))
        _
        (else
          (Components|Movement|StopMovementImmediately _charactermovement)
          (Variables|/Script/Engine.CharacterMovementComponent|SetGravityScale _charactermovement 0.0)
          (Input|SetIgnoreMoveInput (Variables|Default|GetControllerRef) false)))
      (bind _hatref_2 (Variables|Hat|GetHatRef)
        (:then
          (EventDispatchers|BindEventtoOnHatReturned _hatref_2 (delegate Custom|OnHatReturned))
          (EventDispatchers|BindEventtoOnHatBeingJumpedbyPlayer _hatref_2 (delegate Custom|PerformHatJump))
          (Transformation|DetachFromActor (Variables|Hat|GetHatRef) "KeepWorld" "KeepWorld" "KeepWorld")
          (EventDispatchers|BindEventtoOnHatReachedPossessablePawn _hatref_2 (delegate Custom|TryPossessPawn))
          (Transformation|SetActorRotation (Variables|Hat|GetHatRef) (Math|Rotator|MakeRotfromX (Transformation|GetActorForwardVector)))
          (Default|LaunchHat (Variables|Hat|GetHatRef) self)
          (Utilities|FlowControl|Delay 0.2)
          (Variables|/Script/Engine.CharacterMovementComponent|SetGravityScale (Variables|Character|GetCharacterMovement) (Variables|Jump|GetBaseJumpingGravityFactor))
          (bind _controllerref (Variables|Default|GetControllerRef)
            (:then
              (Input|ResetIgnoreMoveInput _controllerref))
            (:else)))
        (:else)))
    (else
      (Default|HatReturn _hatref))))

(event EventUnSmash
  (Character|UnCrouch))

(event EventPossessed
  (params (NewController :type Controller%20Object%20Reference))
  (bind _aspc_player_base (Utilities|Casting|CastToPC_PlayerBase NewController))
  (Variables|Default|SetControllerRef _aspc_player_base)
  (EventDispatchers|BindEventtoOnControlSchemeChanged _aspc_player_base (delegate Custom|ControlSchemeChanged)))

(event EventTick
  (params (DeltaSeconds :type Float%20%28single-precision%29))
  (Utilities|TryAutoAdjustCamRotationonGround))

(event EventUnJump
  (Character|StopJumping))

(event EventStartJump
  (bind _returnvalue (Transformation|GetActorLocation))
  (bind _controllerref (Variables|Default|GetControllerRef)
    (:then
      (switch Utilities|FlowControl|Switch|SwitchonEnum_ControlScheme (Default|GetControlScheme _controllerref)
        (:NewEnumerator0
          (Character|Jump))
        (:NewEnumerator2
          (bind _outhits (Collision|MultiLineTraceByChannel _returnvalue (+ _returnvalue (* (Transformation|GetActorForwardVector) 1e+02)) "TraceTypeQuery1" false 0 "Persistent"))
          (Variables|/Script/Engine.CharacterMovementComponent|SetGravityScale (Variables|Character|GetCharacterMovement) (Variables|Jump|GetBaseJumpingGravityFactor))
          (Transformation|SetActorRotation (Math|Rotator|MakeRotator 0.0 0.0 (.yaw (Math|Rotator|MakeRotfromX (Math|Vector|Normalize (+ (.impactnormal (Utilities|Array|Get(acopy) _outhits)) "0,0,0.200000"))))))
          (Character|LaunchCharacter (* (Math|Vector|Normalize (+ (.impactnormal (Utilities|Array|Get(acopy) _outhits)) "0,0,0.200000")) 1e+03) true true))))
    (:else)))

(event EventMoveRight
  (params (axisVal :type Float%20%28double-precision%29))
  (Pawn|Input|AddMovementInput (.NormalizedRhtVector (CallFunction|GetComponentXYPlaneVector (Variables|Default|GetCamera))) axisVal false))

(event EventMoveForward
  (params (axisVal :type Float%20%28double-precision%29))
  (Pawn|Input|AddMovementInput (.NormalizedFwdVector (CallFunction|GetComponentXYPlaneVector (Variables|Default|GetCamera))) axisVal false))

(event EventLookRight
  (params (axisVal :type Float%20%28double-precision%29))
  (Transformation|AddRelativeRotation (Variables|Default|GetSpringArm) (Math|Rotator|MakeRotator 0.0 0.0 axisVal) false false))

(event EventLookUp
  (params (axisVal :type Float%20%28double-precision%29))
  (Transformation|AddRelativeRotation (Variables|Default|GetSpringArm) (Math|Rotator|MakeRotator 0.0 axisVal 0.0) false false))

(event EventSmash
  (bind _charactermovement (Variables|Character|GetCharacterMovement))
  (bind _controllerref (Variables|Default|GetControllerRef)
    (:then
      (switch Utilities|FlowControl|Switch|SwitchonEnum_ControlScheme (Variables|/Game/Blueprints/Controller/PC_PlayerBase.PC_PlayerBase_C|GetCurrentControlScheme _controllerref)
        (:NewEnumerator0
          (Character|Crouch))
        (:NewEnumerator1
          (if (CallFunction|CanSmash)
            (Input|SetIgnoreMoveInput _controllerref true)
            (Variables|Smash|SetInSmash true)
            (Components|Movement|StopMovementImmediately _charactermovement)
            (Variables|/Script/Engine.CharacterMovementComponent|SetGravityScale _charactermovement 0.0)
            (Utilities|FlowControl|Delay 0.5)
            (CallFunction|SmashDown)
            (EventDispatchers|BindEventtoOnControlSchemeChanged _controllerref (delegate Custom|ResetSmashControlSchemeListener))))))
    (:else)))

(fn ConstructionScript)

(fn GetComponentXYPlaneVector
  (params (ActorComp :type Scene%20Component%20Object%20Reference))
  (bind _returnvalue (Math|Vector|GetForwardVector ActorComp))
  (bind _returnvalue_2 (Math|Vector|GetRightVector ActorComp))
  (return (Math|Vector|Normalize (Math|Vector|MakeVector (.x _returnvalue) (.y _returnvalue) 0.0)) (Math|Vector|Normalize (Math|Vector|MakeVector (.x _returnvalue_2) (.y _returnvalue_2) 0.0))))

(fn SmashDown
  (Character|LaunchCharacter "0, 0,-2000.000000" true true))

(fn CanRollForward
  (return (and (not (Variables|Smash|GetInSmash)) (not (Variables|RollFoward|GetInRollForward)))))

(fn CanSmash
  (return (not (Variables|Smash|GetInSmash))))

(fn ResetSmash
  (Variables|Smash|SetInSmash false))

(fn CanTriggerHat
  (bind _charactermovement (Variables|Character|GetCharacterMovement))
  (return (Math|Boolean|ANDBoolean (not (Variables|Default|GetbIsCrouched)) (not (Variables|Smash|GetInSmash)) (or (AI|Components|NavMovement|IsFalling _charactermovement) (AI|Components|NavMovement|IsMovingonGround _charactermovement)) (Variables|/Game/Blueprints/Actor/BPA_Hat_Base.BPA_Hat_Base_C|GetIsHatReady (Variables|Hat|GetHatRef)) (not (Default|GetonWall (Variables|Default|GetControllerRef))))))

(fn ResetRollForward
  (Variables|RollFoward|SetInRollForward false))

(fn InitializeCameraRotation
  (bind _meshfwddebugvector (Variables|Default|GetMeshFwdDebugVector))
  (bind _returnvalue (Math|Vector|GetForwardVector _meshfwddebugvector))
  (Transformation|SetRelativeRotation (Variables|Default|GetSpringArm) (Math|Rotator|MakeRotfromX (Math|Vector|Normalize (Math|Vector|MakeVector (.x _returnvalue) (.y _returnvalue) (- (.z _returnvalue) (Variables|/Game/Blueprints/GameInstance/GI_Mario.GI_Mario_C|GetAutoCamAdjustmentStableZ (CallFunction|GetMarioGameInstance)))))) false false))