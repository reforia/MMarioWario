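; Possessable switch character whose lever the player tilts while possessing it.
; MoveRight adds the axis value to SwitchRoot's relative roll, zeroing pitch and yaw.
; The rotation only applies while the resulting absolute roll stays below MaxRollableAngle.
; BeginPlay, overlap and Tick hold only disabled stub nodes.
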(event EventBeginPlay
  (|CallParentFunction) ; This node is disabled and will not be called.\nDrag off pins to build functionality.
)

(event Collision|EventActorBeginOverlap
  (params (OtherActor :type Actor%20Object%20Reference))
  (|CallParentFunction OtherActor) ; This node is disabled and will not be called.\nDrag off pins to build functionality.
)

(event EventTick
  (params (DeltaSeconds :type Float%20%28single-precision%29))
  (|CallParentFunction DeltaSeconds) ; This node is disabled and will not be called.\nDrag off pins to build functionality.
)

(event EventMoveRight
  (params (axisVal :type Float%20%28double-precision%29))
  (bind _switchroot (Variables|Default|GetSwitchRoot))
  (bind _relativerotation (Variables|/Script/Engine.SceneComponent|GetRelativeRotation _switchroot))
  (bind _returnvalue (+ (.roll _relativerotation) axisVal))
  (if (< (Math|Float|Absolute(Float) _returnvalue) (Variables|Default|GetMaxRollableAngle))
    (Transformation|SetRelativeRotation _switchroot (Math|Rotator|MakeRotator _returnvalue 0.0 0.0) false false)))

(fn ConstructionScript
  (|CallParentFunction))