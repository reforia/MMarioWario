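; Base Blueprint for possessable characters, providing camera look control and a hat launch that hands control to a player character.
; LookUp and LookRight rotate the SpringArm in pitch and yaw while CanControlCamera is set.
; LaunchHat spawns a Char_PlayerBase at this actor's location projected onto the navmesh, then attempts to possess it through TryPossessTarget.
; The Possessed event is an empty stub.
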(event EventBeginPlay)

(event Collision|EventActorBeginOverlap
  (params (OtherActor :type Actor%20Object%20Reference)))

(event EventTick
  (params (DeltaSeconds :type Float%20%28single-precision%29)))

(event EventPossessed
  (params (NewController :type Controller%20Object%20Reference)))

(event EventLaunchHat
  (bind _returnvalue (Transformation|GetActorTransform))
  (bind _returnvalue_2 (Game|SpawnActorfromClass "/Game/Blueprints/Character/Char_PlayerBase.Char_PlayerBase_C" (Math|Transform|MakeTransform (.ProjectedLocation (AI|Navigation|ProjectPointtoNavigation (.location _returnvalue) 0 0 "500.000000,500.000000,500.000000")) (.rotation _returnvalue) (.scale _returnvalue)) "Undefined" 0 (Game|GetPlayerCharacter 0)))
  (CallFunction|TryPossessTarget _returnvalue_2))

(event EventLookRight
  (params (axisVal :type Float%20%28double-precision%29))
  (if (Variables|Default|GetCanControlCamera)
    (Transformation|AddRelativeRotation (Variables|Default|GetSpringArm) (Math|Rotator|MakeRotator 0.0 0.0 axisVal) false false)))

(event EventLookUp
  (params (axisVal :type Float%20%28double-precision%29))
  (if (Variables|Default|GetCanControlCamera)
    (Transformation|AddRelativeRotation (Variables|Default|GetSpringArm) (Math|Rotator|MakeRotator 0.0 axisVal 0.0) false false)))

(fn ConstructionScript)