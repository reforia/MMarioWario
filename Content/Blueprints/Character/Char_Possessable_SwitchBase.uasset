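; Base possessable switch that notifies linked response actors when triggered and can limit control afterward.
; Components are registered with default and triggered transforms; untriggered ones can spring back to default through interpolation on Tick.
; Reaching the threshold fires the one-time trigger, then a timeline lerps components to their triggered transforms and pops the player out.
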(event Custom|SwitchTriggered
  (if (not (Variables|Default|GetIsTriggered))
    (Variables|Default|SetIsTriggered true)
    (Default|CallOnSwitchTriggered)
    (for _array_element (Variables|Default|GetControlledTriggerResponseActors)
      (Class|BPITriggerResponse|ControllerTriggered(Message) _array_element true))))

(event Custom|TriggerThresholdReached
  (bind _registeredcomponenttriggeredtransform (Variables|Default|GetRegisteredComponentTriggeredTransform))
  (CallFunction|SwitchTriggered)
  (bind _proportiontotarget (Timeline|SnapToDestination Play)
    (:Update
      (bind _keys (Utilities|Map|Keys _registeredcomponenttriggeredtransform))
      (for _array_element _keys
        (if (.ReturnValue (Utilities|Map|Find _registeredcomponenttriggeredtransform _array_element))
          (Transformation|SetRelativeTransform _array_element (Math|Transform|MakeTransform (.location (Math|Transform|Lerp(Transform) (Transformation|GetRelativeTransform _array_element) (.Value (Utilities|Map|Find _registeredcomponenttriggeredtransform _array_element)) _proportiontotarget)) (.rotation (Math|Transform|Lerp(Transform) (Transformation|GetRelativeTransform _array_element) (.Value (Utilities|Map|Find _registeredcomponenttriggeredtransform _array_element)) _proportiontotarget)) "1.000000,1.000000,1.000000") false false))))
    (:Finished
      (CallFunction|PopOutPlayer))))

(event EventBeginPlay)

(event Collision|EventActorBeginOverlap
  (params (OtherActor :type Actor%20Object%20Reference)))

(event EventTick
  (params (DeltaSeconds :type Float%20%28single-precision%29))
  (bind _returnvalue (Utilities|Time|GetWorldDeltaSeconds))
  (bind _registeredcomponentdefaulttransform (Variables|Default|GetRegisteredComponentDefaultTransform))
  (bind _returnbackfriction (Variables|Default|GetReturnBackFriction))
  (if (and (Variables|Default|GetSpringReturnToDefaultTransformWhenNotTrigger) (not (Variables|Default|GetIsTriggered)))
    (bind _keys (Utilities|Map|Keys _registeredcomponentdefaulttransform))
    (for _array_element _keys
      (if (.ReturnValue (Utilities|Map|Find _registeredcomponentdefaulttransform _array_element))
        (Transformation|SetRelativeTransform _array_element (Math|Transform|MakeTransform (Math|Interpolation|VInterpTo (.location (Transformation|GetRelativeTransform _array_element)) (.location (.Value (Utilities|Map|Find _registeredcomponentdefaulttransform _array_element))) _returnvalue _returnbackfriction) (Math|Interpolation|RInterpTo (.rotation (Transformation|GetRelativeTransform _array_element)) (.rotation (.Value (Utilities|Map|Find _registeredcomponentdefaulttransform _array_element))) _returnvalue _returnbackfriction) "1.000000,1.000000,1.000000") false false)))))

(fn ConstructionScript)

(fn GetCanControl
  (return (or (and (Variables|Default|GetCanUseAfterTriggered) (Variables|Default|GetIsTriggered)) (not (Variables|Default|GetIsTriggered)))))

(fn SetDefaultTransform
  (params (Component :type Scene%20Component%20Object%20Reference))
  (if (Utilities|IsValid Component)
    (Utilities|Map|Add (Variables|Default|GetRegisteredComponentDefaultTransform) Component (Transformation|GetRelativeTransform Component))))

(fn SetTriggeredTransform
  (params (SceneComp :type Scene%20Component%20Object%20Reference) (TriggeredTransform :type Transform))
  (if (Utilities|IsValid SceneComp)
    (Utilities|Map|Add (Variables|Default|GetRegisteredComponentTriggeredTransform) SceneComp TriggeredTransform)))