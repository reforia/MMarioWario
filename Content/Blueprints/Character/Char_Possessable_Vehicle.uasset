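; Possessable vehicle Blueprint that turns movement axis events into driving input for a Chaos wheeled vehicle movement component.
; MoveForward passes its axis value to IncreaseThrottleInput, and MoveRight sets steering directly, with no brake or reverse handling in this graph.
; The Possessed event is an empty stub, the default lifecycle events are disabled, and construction only calls the parent script.
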(event EventBeginPlay
  (|CallParentFunction) ; This node is disabled and will not be called.\nDrag off pins to build functionality.
)

(event Collision|EventActorBeginOverlap
  (params (OtherActor :type Actor%20Object%20Reference))
  (|CallParentFunction OtherActor) ; This node is disabled and will not be called.\nDrag off pins to build functionality.
)

(event EventTick
  (params (DeltaSeconds :type Float%20%28single-precision%29))
  (|CallParentFunction DeltaSeconds) ; This node is disabled and will not be called.\nDrag off pins to build functionality.
)

(event EventMoveForward
  (params (axisVal :type Float%20%28double-precision%29))
  (Class|ChaosVehicleMovementComponent|IncreaseThrottleInput (Variables|Default|GetChaosWheeledVehicleMovement) axisVal))

(event EventMoveRight
  (params (axisVal :type Float%20%28double-precision%29))
  (Class|ChaosVehicleMovementComponent|SetSteeringInput (Variables|Default|GetChaosWheeledVehicleMovement) axisVal))

(event EventPossessed
  (params (NewController :type Controller%20Object%20Reference)))

(fn ConstructionScript
  (|CallParentFunction))