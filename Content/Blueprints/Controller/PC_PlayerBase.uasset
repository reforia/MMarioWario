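; Base player controller that turns player input into interface messages on the possessed pawn and handles blended possession switches to a new target.
; Each tick it derives a control scheme from the character's movement state, using a forward trace for wall detection, and ignores move input on walls.
; In the normal game state it forwards axes every tick, while action inputs are stored as flags and edge-detected by a macro to send press and release messages.
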(event Custom|OnReceivedPossesionRequest
  (params (Target :type Pawn%20Object%20Reference))
  (bind _possessionblendtime (Variables|Default|GetPossessionBlendTime))
  (Game|Player|SetViewTargetwithBlend Target _possessionblendtime "VTBlend_EaseInOut" 2.0 false)
  (Utilities|FlowControl|Delay _possessionblendtime)
  (Pawn|UnPossess)
  (Pawn|Possess Target))

(event EventBeginPlay)

(event EventTick
  (params (DeltaSeconds :type Float%20%28single-precision%29))
  (Utilities|FlowControl|Sequence
    (:then_0
      (CallFunction|EvaluateControlScheme))
    (:then_1
      (switch Utilities|FlowControl|Switch|SwitchonEnum_GameStates (CallFunction|GetCurrentGameState)
        (:NewEnumerator1
          (Utilities|NormalControlScheme))))))

(event EventPossess
  (params (PossessedPawn :type Pawn%20Object%20Reference))
  ;[1 1 1] Initial Possession
  (Variables|Default|SetPossessedPawn PossessedPawn))

(event EventUnPossess
  (params (UnpossessedPawn :type Pawn%20Object%20Reference))
  ;[1 1 1] Initial Possession
  (Variables|Default|SetPossessedPawn 0))

(event Input|ActionEvents|InputActionLaunchHat
  (params (Key :type Key%20Structure :default "None"))
  ;[1 1 1] Normal Input Action State
  (:Pressed
    (Variables|Default|SetLaunchHatPressed true))
  (:Released
    (Variables|Default|SetLaunchHatPressed false)))

(event Input|ActionEvents|InputActionRollForward
  (params (Key :type Key%20Structure :default "None"))
  ;[1 1 1] Normal Input Action State
  (:Pressed
    (Variables|Default|SetRollForwardPressed true))
  (:Released
    (Variables|Default|SetRollForwardPressed false)))

(event Input|ActionEvents|InputActionSmash
  (params (Key :type Key%20Structure :default "None"))
  ;[1 1 1] Normal Input Action State
  (:Pressed
    (Variables|Default|SetSmashPressed true))
  (:Released
    (Variables|Default|SetSmashPressed false)))

(event Input|ActionEvents|InputActionJump
  (params (Key :type Key%20Structure :default "None"))
  ;[1 1 1] Normal Input Action State
  (:Pressed
    (Variables|Default|SetJumpPressed true))
  (:Released
    (Variables|Default|SetJumpPressed false)))

(event Input|AxisEvents|InputAxisMoveForward
  (params (AxisValue :type Float%20%28single-precision%29))
  ;[1 1 1] Equivalent Axis Input
)

(event Input|AxisEvents|InputAxisMoveRight
  (params (AxisValue :type Float%20%28single-precision%29))
  ;[1 1 1] Equivalent Axis Input
)

(fn ConstructionScript)

(fn GetInputAnalogDir
  (return (Math|Vector2D|Normalize2D (Math|Vector2D|MakeVector2D (Input|AxisValues|GetMoveForward) (Input|AxisValues|GetMoveRight)))))

(fn SetControlScheme
  (params (NewControlScheme :type Enum_ControlScheme%20Enum :default "NewEnumerator0"))
  (if (Utilities|Enum|NotEqual(Enum) NewControlScheme (CallFunction|GetControlScheme))
    (bind _output_get (Variables|Default|SetCurrentControlScheme NewControlScheme))
    (Default|CallOnControlSchemeChanged _output_get)
    (CallFunction|InitializeControlScheme)))

(fn GetControlScheme
  (return (Variables|Default|GetCurrentControlScheme)))

(fn EvaluateControlScheme
  (bind _ascharacter (Utilities|Casting|CastToCharacter (Variables|Default|GetPossessedPawn))
    (:then
      (CallFunction|SetControlScheme (select (AI|Components|NavMovement|IsMovingonGround (Variables|/Script/Engine.Character|GetCharacterMovement _ascharacter)) "NewEnumerator0" (select (Class|NavMovementComponent|IsFlying (Variables|/Script/Engine.Character|GetCharacterMovement _ascharacter)) "NewEnumerator3" (select (CallFunction|GetonWall) "NewEnumerator2" (select (AI|Components|NavMovement|IsFalling (Variables|/Script/Engine.Character|GetCharacterMovement _ascharacter)) "NewEnumerator1" "NewEnumerator4")))))
      (Development|PrintString (Utilities|String|EnumtoString (select (AI|Components|NavMovement|IsMovingonGround (Variables|/Script/Engine.Character|GetCharacterMovement _ascharacter)) "NewEnumerator0" (select (Class|NavMovementComponent|IsFlying (Variables|/Script/Engine.Character|GetCharacterMovement _ascharacter)) "NewEnumerator3" (select (CallFunction|GetonWall) "NewEnumerator2" (select (AI|Components|NavMovement|IsFalling (Variables|/Script/Engine.Character|GetCharacterMovement _ascharacter)) "NewEnumerator1" "NewEnumerator4"))))) true true "(R=1.000000,G=1.000000,B=0.000000,A=1.000000)" 0.0))
    (:CastFailed
      (Development|PrintString "Possessed Pawn is Not A Character! Evaluate Control Scheme Failed" true true "(R=1.000000,G=0.000000,B=0.000000,A=1.000000)" 0.0))))

(fn GetonWall
  (bind _possessedpawn (Variables|Default|GetPossessedPawn))
  (bind _returnvalue (Transformation|GetActorLocation _possessedpawn))
  (bind _ascharacter (Utilities|Casting|CastToCharacter _possessedpawn))
  (if (AI|Components|NavMovement|IsFalling (Variables|/Script/Engine.Character|GetCharacterMovement _ascharacter))
    (bind (_outhit _returnvalue_2) (Collision|LineTraceByChannel _returnvalue (+ _returnvalue (* (Transformation|GetActorForwardVector _possessedpawn) 7e+01)) "TraceTypeQuery1" false 0 "None"))
    (Variables|Default|SetOnWallNormal (.normal _outhit))
    (return (and _returnvalue_2 (== (.physmat _outhit) 0)))))

(fn InitializeControlScheme
  (switch Utilities|FlowControl|Switch|SwitchonEnum_ControlScheme (CallFunction|GetControlScheme)
    (:NewEnumerator0
      (Input|SetIgnoreMoveInput false))
    (:NewEnumerator1
      (Input|SetIgnoreMoveInput false))
    (:NewEnumerator3
      (Input|SetIgnoreMoveInput false))
    (:NewEnumerator2
      (Input|SetIgnoreMoveInput true))))