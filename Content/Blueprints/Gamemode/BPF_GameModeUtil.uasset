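; Blueprint function library giving world-context access to the Mario game mode, game instance and current game state.
; Getter functions cast to GM_Mario and GI_Mario, printing a red on-screen error when a cast fails.
; The game state query reads from the game mode, falling back to a default enum value if it is invalid.
; A helper reports whether normal movement is allowed by comparing that state to one enum value.
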(fn GetCurrentGameState
  (bind ___worldcontext (LocalVariables|Get__WorldContext))
  (bind _gmref (CallFunction|GetMarioGameMode ___worldcontext))
  (Utilities|IsValid _gmref
    (:Is%20Valid
      (bind _currentgamestate (Default|GetGameState _gmref))
      (return _currentgamestate))
    (:Is%20Not%20Valid
      (return "NewEnumerator6"))))

(fn GetIsAllowNormalMovement
  (return (Utilities|Enum|Equal(Enum) (CallFunction|GetCurrentGameState (LocalVariables|Get__WorldContext)) "NewEnumerator1")))

(fn GetMarioGameMode
  (bind _asgm_mario (Utilities|Casting|CastToGM_Mario (Game|GetGameMode (LocalVariables|Get__WorldContext)))
    (:then
      (return _asgm_mario))
    (:CastFailed
      (Development|PrintString 0 "FAILED TO CAST GAME MODE, DID IT BEING SET CORRECTLY?" true true "(R=1.000000,G=0.000000,B=0.000000,A=1.000000)" 1e+01)
      (return 0))))

(fn GetMarioGameInstance
  (bind ___worldcontext (LocalVariables|Get__WorldContext))
  (bind _asgi_mario (Utilities|Casting|CastToGI_Mario (Game|GetGameInstance ___worldcontext))
    (:then
      (return _asgi_mario))
    (:CastFailed
      (Development|PrintString ___worldcontext "FATAL ERROR!!! THE GI WASN\"T ASSIGNED CORRECTLY!" true true "(R=1.000000,G=0.000000,B=0.000000,A=1.000000)" 1e+01))))