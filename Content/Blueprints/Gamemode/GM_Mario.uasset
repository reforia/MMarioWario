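; Mario game mode that tracks the current game state and spawns a player character on request.
; SetGameState stores a new state and fires the state-changed dispatcher only when the value differs; PostLogin sets an initial test state.
; PopBackToPlayerCharater spawns a Char_PlayerBase slightly above the nav-mesh projection of the given pawn's location, keeping its rotation, and attempts to possess it.
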(event Custom|PopBackToPlayerCharater
  (params (FromPawn :type Pawn%20Object%20Reference))
  (bind _returnvalue (Transformation|GetActorTransform FromPawn))
  (bind _returnvalue_2 (Game|SpawnActorfromClass "/Game/Blueprints/Character/Char_PlayerBase.Char_PlayerBase_C" (Math|Transform|MakeTransform (+ (.ProjectedLocation (AI|Navigation|ProjectPointtoNavigation (.location _returnvalue) 0 0 "500.000000,500.000000,500.000000")) "0,0,100.000000") (.rotation _returnvalue) "1.000000,1.000000,1.000000") "AdjustIfPossibleButAlwaysSpawn" 0 0))
  (CallFunction|TryPossessTarget _returnvalue_2))

(event EventBeginPlay)

(event EventTick
  (params (DeltaSeconds :type Float%20%28single-precision%29)))

(event EventPostLogin
  (params (NewPlayer :type Player%20Controller%20Object%20Reference))
  ;[1 1 1] Test Initialization
  (CallFunction|SetGameState "NewEnumerator1"))

(fn ConstructionScript)

(fn SetGameState
  (params (NewGameState :type Enum_GameStates%20Enum :default "NewEnumerator0"))
  (if (Utilities|Enum|NotEqual(Enum) NewGameState (Variables|Default|GetCurrentGameState))
    (bind _output_get (Variables|Default|SetCurrentGameState NewGameState))
    (Default|CallOnGameStateChanged _output_get)))

(fn GetGameState
  (return (Variables|Default|GetCurrentGameState)))